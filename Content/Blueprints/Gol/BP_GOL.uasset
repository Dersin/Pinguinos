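; BP_GOL is a goal trigger actor for a two-player game scored with a disc.
; When a BP_Disco overlaps its Box component, PlayerGoal selects which player's score to increment in GI_Game, with zero crediting player one and any other value player two.
; It then reloads ThirdPersonMap by name, with the score held in the game instance so it survives the level restart.
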(event OnComponentBeginOverlap(Box)
  (params (OverlappedComponent :type Primitive%20Component%20Object%20Reference) (OtherActor :type Actor%20Object%20Reference) (OtherComp :type Primitive%20Component%20Object%20Reference) (OtherBodyIndex :type Integer) (bFromSweep :type Boolean) (SweepResult :type Hit%20Result%20Structure%20%28by%20ref%29))
  (Utilities|Casting|CastToBP_Disco OtherActor)
  (if (== (Variables|Default|GetPlayerGoal) 0)
    (bind _asgi_game (Utilities|Casting|CastToGI_Game (Game|GetGameInstance)))
    (Math|Integer|IncrementInt (Variables|/Game/Core/GI_Game.GI_Game_C|GetScorePlayer1 _asgi_game)
      (:%20%20
        (Game|OpenLevel(byName) "ThirdPersonMap")))
    (else
      (bind _asgi_game_2 (Utilities|Casting|CastToGI_Game (Game|GetGameInstance)))
      (Math|Integer|IncrementInt (Variables|/Game/Core/GI_Game.GI_Game_C|GetScorePlayer2 _asgi_game_2)
        (:%20%20
          (Game|OpenLevel(byName) "ThirdPersonMap"))))))

(event EventBeginPlay)

(event Collision|EventActorBeginOverlap
  (params (OtherActor :type Actor%20Object%20Reference)))

(event EventTick
  (params (DeltaSeconds :type Float%20%28single-precision%29)))

(fn ConstructionScript)