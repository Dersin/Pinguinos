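; BP_Spawner is a spawner that keeps placing random actors at random target points throughout play.
; From BeginPlay, the SpawnItem event loops by calling itself after a fixed delay and picking a random entry from Targets.
; It spawns a random ActorsToSpawn class at that target's sprite transform, unless the target matches the last one used.
; A repeat pick skips that cycle and waits through another delay.
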(event Custom|SpawnItem
  (Utilities|FlowControl|Delay 5.0)
  (Variables|Default|SetTargetToSpawn (.OutItem (Utilities|Array|Random (Variables|Default|GetTargets))))
  (if (!= (Variables|Default|GetLastSpawnter) (Variables|Default|GetTargetToSpawn))
    (Game|SpawnActorfromClass (.OutItem (Utilities|Array|Random (Variables|Default|GetActors_To_Spawn))) (Transformation|GetWorldTransform (Variables|/Script/Engine.TargetPoint|GetSpriteComponent (Variables|Default|GetTargetToSpawn))) "Undefined" "MultiplyWithRoot" 0 0)
    (Variables|Default|SetLastSpawnter (Variables|Default|GetTargetToSpawn))
    (CallFunction|SpawnItem)
    (else
      (CallFunction|SpawnItem))))

(event EventBeginPlay
  (CallFunction|SpawnItem))

(fn ConstructionScript)